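; Dialog actor that lets a player open a conversation window by interacting with it.
; One second after BeginPlay it names its Dialog component "Test" and initializes it from a fixed ID.
; Interaction passes the component and the actor to the PlayerController's dialog window call.
; Getter functions expose the component and a hard-coded relation value, and map a given relation to an attitude label by thresholds.
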(event EventBeginPlay
  (Utilities|FlowControl|Delay 1.0)
  (Variables|/Script/DialogAndQuestPlugin.DialogComponent|SetDialogName (Variables|Default|GetDialog) "Test")
  (Class|DialogComponent|InitDialogfromID (Variables|Default|GetDialog) 1))

(event Collision|EventActorBeginOverlap
  (params (OtherActor :type Actor%20Object%20Reference)))

(event EventOnInteraction
  (params (PlayerController :type BP%20Dialog%20Player%20Controller%20Object%20Reference))
  (Class|DialogDisplayInterface|CreateDialogWindow(Message) PlayerController (Variables|Default|GetDialog) self))

(fn ConstructionScript)

(fn BPGetDialogComponent
  (return (Variables|Default|GetDialog)))

(fn BPGetRelation
  (return (Variables|Default|GetHardCodedRelation)))

(fn BPGetRelationString
  (params (Relation :type Float%20%28single-precision%29))
  (if (< Relation 0.375)
    (return "Dubious")
    (elif (< Relation 0.4)
      (return "Apprehensively")
      (elif (< Relation 0.6)
        (return "Indifferently")
        (else
          (return "Amiably"))))))