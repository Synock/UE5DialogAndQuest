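; Player controller for a dialog and quest system, handling interaction input and the related UI.
; BeginPlay creates the main HUD and hidden quest journal only on the Remote authority branch, and J toggles the journal, input mode and cursor.
; E traces from the camera and calls BP_InteractionInterface on the hit actor, falling back to its components.
; CreateDialogWindow opens a dialog widget in UI-only input, and TriggerDialogOption forwards topics to it.
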(event EventBeginPlay
  (Networking|SwitchHasAuthority
    (:Remote
      (bind _returnvalue (UserInterface|CreateWidget "/Game/UI_MainHUD.UI_MainHUD_C" self))
      (bind _output_get (Variables|Default|SetMainHud _returnvalue))
      (UserInterface|Viewport|AddtoViewport _output_get 0)
      (bind _returnvalue_2 (UserInterface|CreateWidget "/DialogAndQuestPlugin/UI/QuestJournal/UI_QuestJournal.UI_QuestJournal_C" self))
      (bind _output_get_2 (Variables|Default|SetQuestJournal _returnvalue_2))
      (UserInterface|Viewport|AddtoViewport _output_get_2 0)
      (Widget|SetVisibility (Variables|Default|GetQuestJournal) "Hidden")
      ;[1 1 1] UI specific stuff
      (Class|UserWidget|SetDesiredSizeinViewport (Variables|Default|GetQuestJournal) "(X=706.000000,Y=481.000000)")
      (Class|UserWidget|SetPositioninViewport (Variables|Default|GetQuestJournal) (/ (Viewport|GetViewportSize) "(X=2.000000,Y=2.000000)") false))))

(event EventTick
  (params (DeltaSeconds :type Float%20%28single-precision%29)))

(event EventTriggerDialogOption
  (params (DialogTopic :type String))
  (Class|DialogWindow|DisplayDialogTopicfromString (Variables|Default|GetDialogWindow) DialogTopic))

(event Input|KeyboardEvents|J
  (params (Key :type Key%20Structure :default "None"))
  (:Pressed
    (Utilities|FlowControl|DoOnce false :!label _label
      (:Completed
        (CallFunction|ManageQuestJournalDisplay))))
  (:Released
    (goto _label Reset)))

(event Input|KeyboardEvents|E
  (params (Key :type Key%20Structure :default "None"))
  (bind _playercameramanager (Variables|Default|GetPlayerCameraManager))
  (bind _returnvalue (Camera|GetCameraLocation _playercameramanager))
  (:Pressed
    (Utilities|FlowControl|DoOnce false :!label _label
      (:Completed
        (bind (_outhit _returnvalue_2) (Collision|LineTraceByChannel _returnvalue (+ _returnvalue (* (Math|Vector|GetForwardVector (Camera|GetCameraRotation _playercameramanager)) (Math|Conversions|ToVector(Float) 5e+02))) "TraceTypeQuery1" false 0 "ForDuration"))
        (if _returnvalue_2
          (bind _asbp_interaction_interface (Utilities|Casting|CastToBP_InteractionInterface (.HitActor (Collision|BreakHitResult _outhit)))
            (:then
              (Default|OnInteraction _asbp_interaction_interface self)
              (Development|PrintString "Interactable" :!label _label_2))
            (:CastFailed
              (for _array_element (Class|Actor|GetComponentsbyInterface (.HitActor (Collision|BreakHitResult _outhit)) "/Game/BP_InteractionInterface.BP_InteractionInterface_C")
                (Default|OnInteraction (.AsBP%20Interaction%20Interface (Utilities|Casting|CastToBP_InteractionInterface _array_element)) self)
                (goto _label_2))))))))
  (:Released
    (goto _label Reset)))

(fn ConstructionScript)

(fn ManageQuestJournalDisplay
  (Utilities|IsValid (Variables|Default|GetQuestJournal)
    (:Is%20Valid
      (if (Widget|IsVisible (Variables|Default|GetQuestJournal))
        (Widget|SetVisibility (Variables|Default|GetQuestJournal) "Hidden")
        (Input|SetInputModeGameOnly self)
        (Variables|Default|SetbShowMouseCursor false)
        (else
          (Widget|SetVisibility (Variables|Default|GetQuestJournal) "Visible" :!label _label)
          (Input|SetInputModeGameandUI self (Variables|Default|GetQuestJournal) "DoNotLock" true)
          (Variables|Default|SetbShowMouseCursor true))))
    (:Is%20Not%20Valid
      (bind _returnvalue (UserInterface|CreateWidget "/DialogAndQuestPlugin/UI/QuestJournal/UI_QuestJournal.UI_QuestJournal_C" self))
      (bind _output_get (Variables|Default|SetQuestJournal _returnvalue))
      (UserInterface|Viewport|AddtoViewport _output_get 0)
      (goto _label))))

(fn CreateDialogWindow
  (params (DialogComponent :type Dialog%20Component%20Object%20Reference) (DialogActor :type Actor%20Object%20Reference))
  ;[1 1 1] Mandatory initialization
  (bind _returnvalue (UserInterface|CreateWidget "/DialogAndQuestPlugin/UI/UI_DialogWindow.UI_DialogWindow_C" self))
  (bind _output_get (Variables|Default|SetDialogWindow _returnvalue))
  (Class|DialogWindow|InitDialogWindow _output_get DialogComponent DialogActor)
  ;[1 1 1] UI specific stuff
  (Class|UserWidget|SetDesiredSizeinViewport (Variables|Default|GetDialogWindow) "(X=706.000000,Y=481.000000)")
  (Class|UserWidget|SetPositioninViewport (Variables|Default|GetDialogWindow) (/ (Viewport|GetViewportSize) "(X=2.000000,Y=2.000000)") false)
  (UserInterface|Viewport|AddtoViewport (Variables|Default|GetDialogWindow) 0)
  (Input|SetInputModeUIOnly self 0 "DoNotLock")
  (Variables|Default|SetbShowMouseCursor true))

(fn GetDialogWindow
  (return 0))